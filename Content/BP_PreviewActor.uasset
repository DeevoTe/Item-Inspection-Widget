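; BP_PreviewActor is a preview actor that shows a static mesh to a SceneCaptureComponent2D and lets it be rotated and swapped.
; The capture's show-only list holds just this actor, set in both the construction script and BeginPlay.
; RotateMesh orbits the view by adding yaw and inverted pitch deltas to the SpringArm's relative rotation, leaving the mesh itself untouched.
; ChangeMesh cycles through the Meshes array, wrapping to the first after the last.
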(event Custom|Rotate%20Mesh
  (params (Delta%20Rotation%20Y%20%28Pitch%29 :type Float%20%28single-precision%29) (Delta%20Rotation%20Z%20%28Yaw%29 :type Float%20%28single-precision%29))
  (bind _springarm (Variables|Default|GetSpringArm))
  (Transformation|SetRelativeRotation _springarm (Math|Rotator|CombineRotators (Math|Rotator|MakeRotator 0.0 (* Delta%20Rotation%20Y%20%28Pitch%29 -1.0) Delta%20Rotation%20Z%20%28Yaw%29) (Variables|/Script/Engine.SceneComponent|GetRelativeRotation _springarm)) false false))

(event Custom|Change%20Mesh
  (Variables|Default|Seti (select (== (- (Utilities|Array|Length (Variables|Default|GetMeshes)) 1) (Variables|Default|Geti)) 0 (+ (Variables|Default|Geti) 1)))
  (Components|StaticMesh|SetStaticMesh (Variables|Default|GetMesh) (Utilities|Array|Get(acopy) (Variables|Default|GetMeshes) (Variables|Default|Geti))))

(event EventBeginPlay
  (Variables|/Script/Engine.SceneCaptureComponent|SetShowOnlyActors (Variables|Default|GetSceneCaptureComponent2D) (Utilities|Array|MakeArray self)))

(fn ConstructionScript
  (Variables|/Script/Engine.SceneCaptureComponent|SetShowOnlyActors (Variables|Default|GetSceneCaptureComponent2D) (Utilities|Array|MakeArray self)))